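; BP_Item is an item actor with a configurable mesh and floating name label, both applied in the construction script.
; Each tick the label turns to the camera, and a timeline plays while the player is 55–175 units away, otherwise reverses, scaling the text by camera distance.
; PickedUp disables physics and collision, RemoveItem clears the mesh, a DotToPlayer value has accessors, and Thrown is empty.
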(event EventBeginPlay)

(event Collision|EventActorBeginOverlap
  (params (OtherActor :type Actor%20Object%20Reference)))

(event EventTick
  (params (DeltaSeconds :type Float%20%28single-precision%29))
  (bind _returnvalue (Game|GetPlayerCharacter 0))
  (bind _returnvalue_2 (Transformation|GetActorLocation))
  (bind _textrender (Variables|Default|GetTextRender))
  (bind _returnvalue_3 (Transformation|GetActorLocation _returnvalue))
  (bind _returnvalue_4 (- _returnvalue_3 _returnvalue_2))
  (bind _returnvalue_5 (Math|Vector|VectorLength _returnvalue_4))
  (Transformation|SetWorldRotation (Variables|Default|GetTextRender) (Math|Rotator|FindLookatRotation (Transformation|GetActorLocation) (Transformation|GetActorLocation (Game|GetPlayerCameraManager 0))) false false)
  (if (and (> _returnvalue_5 55.0) (< _returnvalue_5 175.0))
    (Rendering|SetVisibility _textrender true false)
    (bind _size (Timeline|Timeline_0 Play)
      (:Update
        (Transformation|SetWorldScale3D (Variables|Default|GetTextRender) (Math|Conversions|ToVector(Float) (* _size (/ (Math|Vector|VectorLength (- (Transformation|GetActorLocation (Game|GetPlayerCameraManager 0)) (Transformation|GetActorLocation))) 5e+02))))))
    (else
      (Rendering|SetVisibility _textrender true false)
      (Timeline|Timeline_0 Reverse))))

(fn ConstructionScript
  (Components|StaticMesh|SetStaticMesh (Variables|Default|GetObjectMesh) (Variables|ItemOptions|GetItemMesh))
  (Rendering|Components|TextRender|SetText (Variables|Default|GetTextRender) (Variables|Default|GetObjectName)))

(fn PickedUp
  (Physics|SetSimulatePhysics (Variables|Default|GetObjectMesh) false)
  (Collision|SetCollisionEnabled (Variables|Default|GetObjectMesh) "NoCollision"))

(fn RemoveItem
  (Components|StaticMesh|SetStaticMesh (Variables|Default|GetObjectMesh) 0))

(fn SetDottoPlayer
  (params (DotToPlayer :type Float%20%28single-precision%29))
  (Variables|Default|SetDotToPlayer DotToPlayer))

(fn GetDottoPlayer
  (return (Variables|Default|GetDotToPlayer)))

(fn Thrown)