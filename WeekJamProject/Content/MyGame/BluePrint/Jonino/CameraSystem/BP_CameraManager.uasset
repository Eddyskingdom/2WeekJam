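; Camera manager actor that controls which follow camera is active for the player.
; On BeginPlay it gathers every BP_FollowCamera and switches to the starting one; SwitchCamera matches by camera name, deactivates the previous camera and passes the new one to the player character.
; After a short delay for UI creation, it looks up the in-game UI widget and shows an interaction prompt.
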(event Custom|DeactivatePreviousCamera
  (bind _activecamera (Variables|Default|GetactiveCamera))
  ;[1 1 1] Disable a camera that is not in use
  (Utilities|IsValid _activecamera
    (:Is%20Valid
      (Default|DeactivateCamera _activecamera))))

(event Custom|SwitchCamera
  (params (CameraName :type CameraNames%20Enum :default "NewEnumerator0"))
  (bind _returnvalue (Game|GetPlayerController 0))
  (bind _returnvalue_2 (Pawn|GetControlledPawn _returnvalue))
  (bind (_asbp_player_character _bsuccess) (Utilities|Casting|CastToBP_PlayerCharacter _returnvalue_2))
  ;[1 1 1] Switch to a camera and deactive
  (bind _array_element (Utilities|Array|ForEachLoopwithBreak (Variables|Default|GetAllCamera's))
    (:LoopBody
      (if (== (Variables|/Game/MyGame/BluePrint/Jonino/CameraSystem/BP_FollowCamera.BP_FollowCamera_C|GetcameraName _array_element) CameraName)
        (CallFunction|DeactivatePreviousCamera)
        (Default|ActivateCamera _array_element)
        (bind _output_get (Variables|Default|SetactiveCamera _array_element))
        (if _bsuccess
          (Default|SetActiveCamera _asbp_player_character _output_get)
          (else
            (Development|PrintString "Could not find the player!" true true "(R=1.000000,G=0.000000,B=0.012647,A=1.000000)" 5.0)))))))

(event EventBeginPlay
  ;[1 1 1] Find all camera's and switch to the starting camera
  (Utilities|FlowControl|Sequence
    (:then_0
      (bind _outactors (Actor|GetAllActorsOfClass "/Game/MyGame/BluePrint/Jonino/CameraSystem/BP_FollowCamera.BP_FollowCamera_C"))
      (bind _output_get (Variables|Default|SetAllCamera's _outactors))
      (Development|PrintString (Utilities|String|Append "[CAMERAMANAGER]: " "Found [" (Utilities|String|ToString(Integer) (Utilities|Array|Length _output_get)) "] Camera's") true true "(R=0.000000,G=0.660000,B=1.000000,A=1.000000)" 1e+01)
      (CallFunction|SwitchCamera (Variables|Default|GetStartingCamera)))
    (:then_1
      (Utilities|FlowControl|Delay 0.1) ; Wait for the player to add UI to the viewport
      (CallFunction|GetIngameUIWidget)
      (Default|ShowInteraction (Variables|Default|GetIngameUI) "NewEnumerator0" "Visible"))))

(fn ConstructionScript)

(fn GetIngameUIWidget
  (bind _foundwidgets (Widget|GetAllWidgetsOfClass "/Game/MyGame/UI/WB_IngameUI.WB_IngameUI_C" true))
  (if (> (Utilities|Array|Length _foundwidgets) 1)
    (Development|PrintString "Multiple UI! [CAMERAMANAGER]" true true "(R=1.000000,G=0.000000,B=0.019224,A=1.000000)" 1e+02)
    (else
      (Utilities|FlowControl|Sequence
        (:then_1
          (Variables|Default|SetIngameUI (Utilities|Array|Get(acopy) _foundwidgets)))))))