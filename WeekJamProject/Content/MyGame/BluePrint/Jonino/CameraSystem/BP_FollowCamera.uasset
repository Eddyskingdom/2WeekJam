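; BP_FollowCamera is a stationary camera actor that turns to track player 0's controlled pawn and supports FOV zooming.
; ActivateCamera blends the player's view to it and enables Tick updates, while DeactivateCamera only stops them.
; While active, it smoothly interpolates pitch and yaw toward the pawn if rotation is enabled.
; ZoomIn and ZoomOut step a clamped target FOV, which Tick eases the camera toward.
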(event Custom|ActivateCamera
  ;[1 1 1] Set Camera in an Active/Inactive state
  (Variables|Default|Setactive true)
  (Game|Player|SetViewTargetwithBlend (Game|GetPlayerController 0) self 0.0 "VTBlend_Linear" 0.0 false))

(event Custom|RotateCamera
  (bind _returnvalue (Transformation|GetActorRotation))
  (bind _returnvalue_2 (Utilities|Time|GetWorldDeltaSeconds))
  (bind _returnvalue_3 (Transformation|GetActorLocation))
  (bind _returnvalue_4 (Game|GetPlayerController 0))
  (bind _returnvalue_5 (Pawn|GetControlledPawn _returnvalue_4))
  (bind _returnvalue_6 (Transformation|GetActorLocation _returnvalue_5))
  (bind _returnvalue_7 (Math|Rotator|FindLookatRotation _returnvalue_3 _returnvalue_6))
  (bind _returnvalue_8 (Math|Interpolation|RInterpTo _returnvalue _returnvalue_7 _returnvalue_2 3.0))
  ;[1 1 1] CameraRotation
  (if (Variables|Default|GetenableRotation)
    (Transformation|SetActorRotation (Math|Rotator|MakeRotator 0.0 (.pitch _returnvalue_8) (.yaw _returnvalue_8)))))

(event Custom|DeactivateCamera
  ;[1 1 1] Set Camera in an Active/Inactive state
  (Variables|Default|Setactive false))

(event Custom|ZoomOut
  (bind _minmaxzoom (Variables|Default|GetminMaxZoom))
  ;[1 1 1] Camera Zooming
  (bind _output_get (Variables|Default|SetzoomValue (+ (Variables|Default|GetzoomValue) 2.5)))
  (Variables|Default|SetzoomValue (Math|Float|Clamp(Float) _output_get (.x _minmaxzoom) (.y _minmaxzoom))))

(event Custom|ZoomIn
  (bind _minmaxzoom (Variables|Default|GetminMaxZoom))
  ;[1 1 1] Camera Zooming
  (bind _output_get (Variables|Default|SetzoomValue (+ (Variables|Default|GetzoomValue) -2.5)))
  (Variables|Default|SetzoomValue (Math|Float|Clamp(Float) _output_get (.x _minmaxzoom) (.y _minmaxzoom))))

(event Custom|Zoom
  ;[1 1 1] Update the FOV of the camera
  (bind _output_get (Variables|Default|SetnewFovValue (Math|Interpolation|FInterpTo (stale _output_get) (Variables|Default|GetzoomValue) (Utilities|Time|GetWorldDeltaSeconds) 3.0)))
  (Camera|SetFieldOfView (Variables|Default|GetCamera) _output_get))

(event EventTick
  (params (DeltaSeconds :type Float%20%28single-precision%29))
  ;[1 1 1] Update Rotation and zooming when active
  (if (Variables|Default|Getactive)
    (Utilities|FlowControl|Sequence
      (:then_0
        (CallFunction|RotateCamera))
      (:then_1
        (CallFunction|Zoom)))))

(fn ConstructionScript)