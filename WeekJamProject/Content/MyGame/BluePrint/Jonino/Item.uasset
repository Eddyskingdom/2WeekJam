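; Item is an actor Blueprint for a world object that can be picked up or cleared.
; The construction script applies the ItemMesh variable to its ObjectMesh component, so each instance can show a different mesh.
; PickedUp disables collision and physics simulation on that mesh, and RemoveItem clears the static mesh without destroying the actor.
; The event graph holds no active logic.
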(event EventBeginPlay)

(event Collision|EventActorBeginOverlap
  (params (OtherActor :type Actor%20Object%20Reference)))

(event EventTick
  (params (DeltaSeconds :type Float%20%28single-precision%29)))

(fn ConstructionScript
  (Components|StaticMesh|SetStaticMesh (Variables|Default|GetObjectMesh) (Variables|ItemOptions|GetItemMesh)))

(fn PickedUp
  (Collision|SetCollisionEnabled (Variables|Default|GetObjectMesh) "NoCollision")
  (Physics|SetSimulatePhysics (Variables|Default|GetObjectMesh) false))

(fn RemoveItem
  (Components|StaticMesh|SetStaticMesh (Variables|Default|GetObjectMesh) 0))