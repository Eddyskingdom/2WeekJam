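; BP_StartCola is a physics prop, apparently a cola object for the game's start, that falls and wakes the player character on impact.
; Its FALL event turns on physics simulation for the static mesh, then after a delay pushes it along the actor's forward vector with an impulse scaled by ImpulsStrength.
; On a hit with BP_PlayerCharacter, it calls that character's WakeUp once through a DoOnce gate.
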(event Custom|FALL
  (bind _returnvalue (Transformation|GetActorLocation))
  (Physics|SetSimulatePhysics (Variables|Default|GetStaticMesh) true)
  (Utilities|FlowControl|Delay 3.5)
  (Physics|AddImpulseatLocation (Variables|Default|GetStaticMesh) (* (Transformation|GetActorForwardVector) (Variables|Default|GetimpulsStrength)) (Math|Vector|MakeVector (.x _returnvalue) (.y _returnvalue) (.z _returnvalue)) "None"))

(event Collision|EventHit
  (params (MyComp :type Primitive%20Component%20Object%20Reference) (Other :type Actor%20Object%20Reference) (OtherComp :type Primitive%20Component%20Object%20Reference) (bSelfMoved :type Boolean) (HitLocation :type Vector :default "0, 0, 0") (HitNormal :type Vector :default "0, 0, 0") (NormalImpulse :type Vector :default "0, 0, 0") (Hit :type Hit%20Result%20Structure%20%28by%20ref%29))
  (bind _asbp_player_character (Utilities|Casting|CastToBP_PlayerCharacter Other))
  (Utilities|FlowControl|DoOnce false
    (:Completed
      (Default|WakeUp _asbp_player_character))))

(fn ConstructionScript)