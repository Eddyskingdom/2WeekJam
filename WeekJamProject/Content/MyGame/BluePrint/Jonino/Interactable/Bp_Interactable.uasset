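; Interactable world object, such as a fridge or dresser, that opens to expose the items inside it.
; BeginPlay builds the parent mesh and skeletal child meshes from a data table row, registering with BP_ItemSpawnManager and fetching contained items inside the per-child loop.
; OpenInteractable enables item overlaps, then per child plays its animation and any matching sound, disables parent overlaps and marks it opened.
; It also stores a DotToPlayer value through a setter and getter.
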(event Custom|OpenInteractable
  (bind _returnvalue (Transformation|GetActorLocation))
  (bind _returnvalue_2 (Utilities|GetDataTableRow "/Game/MyGame/BluePrint/Jonino/Interactable/InteractableObjectData.InteractableObjectData" (Variables|Interactable|GetObjectNameInRow))
    (:then
      (for _array_element (Variables|Default|GetItemsInInteractable)
        (Variables|/Script/Engine.PrimitiveComponent|SetbGenerateOverlapEvents (Variables|/Game/MyGame/BluePrint/Jonino/Item/BP_Item.BP_Item_C|GetObjectMesh _array_element) true))
      (for (_array_element_2 _array_index) (.childmesh _returnvalue_2)
        (Components|Animation|PlayAnimation (Utilities|Array|Get(acopy) (Variables|Default|GetskeletalMeshes) _array_index) (.ChildAnimation (Utilities|Struct|BreakChildMesh _array_element_2)) false)
        (switch name (Variables|Interactable|GetObjectNameInRow)
          (:Fridge
            (Audio|PlaySoundatLocation "/Game/MyGame/Audio/Lisa/fridge-door-open_Cue.fridge-door-open_Cue" _returnvalue "0, 0, 0" 1.0 1.0 0.0 0 0 0))
          (:Dresser
            (Audio|PlaySoundatLocation "/Game/MyGame/Audio/Lisa/fridge-door-open_Cue.fridge-door-open_Cue" _returnvalue "0, 0, 0" 1.0 1.0 0.0 0 0 0)))
        (Variables|/Script/Engine.PrimitiveComponent|SetbGenerateOverlapEvents (Variables|Default|GetParent) false)
        (Variables|Default|SetisOpened true)))))

(event EventBeginPlay
  (bind _returnvalue (Utilities|GetDataTableRow "/Game/MyGame/BluePrint/Jonino/Interactable/InteractableObjectData.InteractableObjectData" (Variables|Interactable|GetObjectNameInRow))
    (:then
      (Components|StaticMesh|SetStaticMesh (Variables|Default|GetParent) (.ParentMesh (Utilities|Struct|BreakInteractableObject _returnvalue)))
      (for _array_element (.ChildMesh (Utilities|Struct|BreakInteractableObject _returnvalue))
        (bind _returnvalue_2 (Game|AddComponentbyClass self "/Script/Engine.SkeletalMeshComponent" false))
        (Class|SkinnedMeshComponent|SetSkeletalMesh _returnvalue_2 (.ChildMesh (Utilities|Struct|BreakChildMesh _array_element)) true)
        (Utilities|Array|Add (Variables|Default|GetskeletalMeshes) _returnvalue_2)
        (bind _returnvalue_3 (Actor|GetActorOfClass "/Game/MyGame/BluePrint/Jonino/Managers/BP_ItemSpawnManager.BP_ItemSpawnManager_C"))
        (Default|RegisterInteractable _returnvalue_3 self)
        (bind _items (Default|GetItemsInteractable _returnvalue_3 (Variables|Default|GetParent)))
        (Variables|Default|SetItemsInInteractable _items)))
    (:RowNotFound
      (Development|PrintString "ROW COULD NOT BE FOUND" true true "(R=1.000000,G=0.000000,B=0.018600,A=1.000000)" 1e+01))))

(fn ConstructionScript
  (Components|StaticMesh|SetStaticMesh (Variables|Default|GetParent) (Variables|Interactable|GetPLACEHOLDER)))

(fn SetDottoPlayer
  (params (Dot :type Float%20%28single-precision%29))
  (Variables|Default|SetdotToPlayer Dot))

(fn GetDottoPlayer
  (return (Variables|Default|GetdotToPlayer)))