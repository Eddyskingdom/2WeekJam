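; BP_PlayerCharacter is the player character, with camera-relative movement, scroll zoom and a countdown shown in the in-game UI.
; Move axes follow the yaw of an externally assigned ActiveCamera, which also handles zooming.
; BeginPlay applies walk speed, sizes the interaction sphere in meters and creates the widget; its overlap events are empty.
; Tick decrements Time and updates the widget, while T sets timer visibility around a retriggerable delay.
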(event OnComponentBeginOverlap(InteractionSphere)
  (params (OverlappedComponent :type Primitive%20Component%20Object%20Reference) (OtherActor :type Actor%20Object%20Reference) (OtherComp :type Primitive%20Component%20Object%20Reference) (OtherBodyIndex :type Integer) (bFromSweep :type Boolean) (SweepResult :type Hit%20Result%20Structure%20%28by%20ref%29)))

(event OnComponentEndOverlap(InteractionSphere)
  (params (OverlappedComponent :type Primitive%20Component%20Object%20Reference) (OtherActor :type Actor%20Object%20Reference) (OtherComp :type Primitive%20Component%20Object%20Reference) (OtherBodyIndex :type Integer)))

(event Custom|SetActiveCamera
  (params (NewCamera :type BP%20Follow%20Camera%20Object%20Reference))
  (Variables|Default|SetactiveCamera NewCamera))

(event Custom|SetUI
  ;[1 1 1] Create UI and add it to the viewport
  (bind _returnvalue (UserInterface|CreateWidget "/Game/MyGame/BluePrint/Jonino/UI/WB_IngameUI.WB_IngameUI_C"))
  (bind _output_get (Variables|Default|SetIngameUI _returnvalue))
  (UserInterface|Viewport|AddtoViewport _output_get 0))

(event Custom|ShowTimeLeft
  (params (Visibility :type ESlateVisibility%20Enum :default "Visible"))
  (bind _ingameui (Variables|Default|GetIngameUI))
  (Default|SetTimeVisibility _ingameui Visibility)
  (Utilities|FlowControl|RetriggerableDelay 2.0)
  (Default|SetTimeVisibility _ingameui "Visible"))

(event EventTick
  (params (DeltaSeconds :type Float%20%28single-precision%29))
  (Utilities|IsValid 0
    (:Is%20Valid
      (Default|UpdateTimeLeft (Variables|Default|GetIngameUI) (Variables|Default|Gettime))
      (Variables|Default|Settime (- (Variables|Default|Gettime) DeltaSeconds)))))

(event EventBeginPlay
  ;[1 1 1] Setup Player
  (Variables|/Script/Engine.CharacterMovementComponent|SetMaxWalkSpeed (Variables|Character|GetCharacterMovement) (Variables|Default|GetmovementSpeed))
  (Components|Sphere|SetSphereRadius (Variables|Default|GetInteractionSphere) (* (Variables|Default|GetInteractionRangeInMeters) 1e+02) true)
  (CallFunction|SetUI))

(event Input|ActionEvents|InputActionScrollUp
  (params (Key :type Key%20Structure :default "None"))
  ;[1 1 1] Zooming
  (:Pressed
    (Utilities|IsValid (Variables|Default|GetactiveCamera)
      (:Is%20Valid
        (Default|Zoomin (Variables|Default|GetactiveCamera))))))

(event Input|ActionEvents|InputActionScrollDown
  (params (Key :type Key%20Structure :default "None"))
  ;[1 1 1] Zooming
  (:Pressed
    (Utilities|IsValid (Variables|Default|GetactiveCamera)
      (:Is%20Valid
        (Default|ZoomOut (Variables|Default|GetactiveCamera))))))

(event Input|AxisEvents|InputAxisMoveForward
  (params (AxisValue :type Float%20%28single-precision%29))
  ;[1 1 1] Movement
  (Pawn|Input|AddMovementInput (Math|Vector|GetForwardVector (Math|Rotator|MakeRotator 0.0 0.0 (.yaw (Transformation|GetActorRotation (Variables|Default|GetactiveCamera))))) AxisValue false))

(event Input|AxisEvents|InputAxisMoveRight
  (params (AxisValue :type Float%20%28single-precision%29))
  ;[1 1 1] Movement
  (Pawn|Input|AddMovementInput (Math|Vector|GetRightVector (Math|Rotator|MakeRotator 0.0 0.0 (.yaw (Transformation|GetActorRotation (Variables|Default|GetactiveCamera))))) AxisValue false))

(event Input|KeyboardEvents|T
  (params (Key :type Key%20Structure :default "None"))
  (:Pressed
    (CallFunction|ShowTimeLeft "Visible")))

(fn ConstructionScript)