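; Settings manager Blueprint that applies four graphics presets: High, Medium, Low and Lowest.
; Each preset event calls functions for shadow quality, screen percentage and post-process anti-aliasing.
; These functions switch on an enum, run the matching console command through player controller 0 and return a level name.
; The Medium resolution option is labeled 85% but sets screen percentage to 75.
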(event Custom|LowestQuality
  (CallFunction|ChangeShadowQuality "NewEnumerator3")
  (CallFunction|ChangeResolution "NewEnumerator3")
  (CallFunction|ChangeAAQuality "NewEnumerator3"))

(event Custom|HighGraphics
  (CallFunction|ChangeShadowQuality "NewEnumerator0")
  (CallFunction|ChangeResolution "NewEnumerator0")
  (CallFunction|ChangeAAQuality "NewEnumerator0"))

(event Custom|MediumGraphics
  (CallFunction|ChangeShadowQuality "NewEnumerator1")
  (CallFunction|ChangeResolution "NewEnumerator1")
  (CallFunction|ChangeAAQuality "NewEnumerator1"))

(event Custom|LowGraphics
  (CallFunction|ChangeShadowQuality "NewEnumerator2")
  (CallFunction|ChangeResolution "NewEnumerator2")
  (CallFunction|ChangeAAQuality "NewEnumerator2"))

(fn ConstructionScript)

(fn ChangeShadowQuality
  (params (Quality :type ShadowQuality%20Enum :default "NewEnumerator0"))
  (bind _returnvalue (Game|GetPlayerController 0))
  (switch Utilities|FlowControl|Switch|SwitchonShadowQuality Quality
    (:NewEnumerator0
      (Development|ExecuteConsoleCommand "r.ShadowQuality 3" _returnvalue)
      (return "High"))
    (:NewEnumerator1
      (Development|ExecuteConsoleCommand "r.ShadowQuality 2" _returnvalue)
      (return "Medium"))
    (:NewEnumerator2
      (Development|ExecuteConsoleCommand "r.ShadowQuality 1" _returnvalue)
      (return "Low"))
    (:NewEnumerator3
      (Development|ExecuteConsoleCommand "r.ShadowQuality 0" _returnvalue)
      (return "Off"))))

(fn ChangeResolution
  (params (Resolution :type ScreenResolution%20Enum :default "NewEnumerator0"))
  (bind _returnvalue (Game|GetPlayerController 0))
  (switch Utilities|FlowControl|Switch|SwitchonScreenResolution Resolution
    (:NewEnumerator0
      (Development|ExecuteConsoleCommand " r.ScreenPercentage 100" _returnvalue)
      (return "High"))
    (:NewEnumerator1
      (Development|ExecuteConsoleCommand " r.ScreenPercentage 75" _returnvalue)
      (return "Medium"))
    (:NewEnumerator2
      (Development|ExecuteConsoleCommand " r.ScreenPercentage 70" _returnvalue)
      (return "Low"))
    (:NewEnumerator3
      (Development|ExecuteConsoleCommand " r.ScreenPercentage 50" _returnvalue)
      (return "Potato"))))

(fn ChangeAAQuality
  (params (Quality :type AAQuality%20Enum :default "NewEnumerator0"))
  (bind _returnvalue (Game|GetPlayerController 0))
  (switch Utilities|FlowControl|Switch|SwitchonAAQuality Quality
    (:NewEnumerator0
      (Development|ExecuteConsoleCommand " r.PostProcessAAQuality 6" _returnvalue)
      (return "High"))
    (:NewEnumerator1
      (Development|ExecuteConsoleCommand " r.PostProcessAAQuality 4" _returnvalue)
      (return "Medium"))
    (:NewEnumerator2
      (Development|ExecuteConsoleCommand " r.PostProcessAAQuality 2" _returnvalue)
      (return "Low"))
    (:NewEnumerator3
      (Development|ExecuteConsoleCommand " r.PostProcessAAQuality 0" _returnvalue)
      (return "Off"))))