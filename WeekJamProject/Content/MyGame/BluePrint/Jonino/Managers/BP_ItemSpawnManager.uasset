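; Manager that spawns random loot and a revolver across furniture and interactable objects in the level.
; Its Get Items functions give each mesh socket a 50% chance of a random-mesh BP_Item, returning those items and caching unused socket locations.
; After a short BeginPlay delay, it places the revolver at a random cached furniture or interactable location.
; An interactable placement also adds the revolver to a randomly picked registered interactable's item list.
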(event Custom|RegisterInteractable
  (params (Interactable :type BP%20Interactable%20Object%20Reference))
  (Utilities|Array|AddUnique (Variables|Default|GetInteractables) Interactable))

(event EventBeginPlay
  (bind _locationsinteractable (Variables|Default|GetLocationsInteractable))
  (bind _locationsfurniture (Variables|Default|GetLocationsFurniture))
  (Utilities|FlowControl|Delay 0.2)
  (Development|PrintString (Utilities|String|Append "SPAWNED [" (Utilities|String|ToString(Integer) (Variables|Default|GetTotalItemsSpawned)) "] Items"))
  (Utilities|FlowControl|Delay 0.5)
  (if (not (Variables|Default|GetspawnedRevolver))
    (switch int (Math|Random|RandomInteger 2)
      (:0
        (bind _returnvalue (Game|SpawnActorfromClass "/Game/MyGame/BluePrint/Jonino/Item/BP_Revolver.BP_Revolver_C" (Math|Transform|MakeTransform (Utilities|Array|Get(acopy) _locationsinteractable (Math|Random|RandomIntegerinRange 0 (- (Utilities|Array|Length _locationsinteractable) 1))) "0, 0, 0" "1,1,1") "AlwaysSpawn" 0 0))
        (bind _output_get (Variables|Default|SetRevolver _returnvalue))
        (Variables|/Script/Engine.PrimitiveComponent|SetbGenerateOverlapEvents (Variables|/Game/MyGame/BluePrint/Jonino/Item/BP_Item.BP_Item_C|GetObjectMesh _output_get) false)
        (Development|PrintString "REVOLVER SPAWNED 2ND CHANCE" true false "(R=0.023822,G=1.000000,B=0.000000,A=1.000000)" 5.0)
        (Utilities|Array|Add (Variables|/Game/MyGame/BluePrint/Jonino/Interactable/Bp_Interactable.BP_Interactable_C|GetItemsInInteractable (Utilities|Array|Get(acopy) (Variables|Default|GetInteractables) (Math|Random|RandomIntegerinRange 0 (Utilities|Array|Length (Variables|Default|GetInteractables))))) (Variables|Default|GetRevolver)))
      (:1
        (bind _returnvalue_2 (Game|SpawnActorfromClass "/Game/MyGame/BluePrint/Jonino/Item/BP_Revolver.BP_Revolver_C" (Math|Transform|MakeTransform (Utilities|Array|Get(acopy) _locationsfurniture (Math|Random|RandomIntegerinRange 0 (- (Utilities|Array|Length _locationsfurniture) 1))) "0, 0, 0" "1,1,1") "AlwaysSpawn" 0 0 :!label _label))
        (bind _output_get_2 (Variables|Default|SetRevolver _returnvalue_2))
        (Variables|/Script/Engine.PrimitiveComponent|SetbGenerateOverlapEvents (Variables|/Game/MyGame/BluePrint/Jonino/Item/BP_Item.BP_Item_C|GetObjectMesh _output_get_2) true)
        (Development|PrintString "REVOLVER SPAWNED 2ND CHANCE" true false "(R=0.023822,G=1.000000,B=0.000000,A=1.000000)" 5.0))
      (:2
        (goto _label)))))

(fn ConstructionScript)

(fn GetItemsFurniture
  (params (Static%20mesh%20component :type Static%20Mesh%20Component%20Object%20Reference))
  (for _array_element (Transformation|GetAllSocketNames Static%20mesh%20component)
    (if (Math|Random|RandomBoolwithWeight 0.5)
      (Utilities|FlowControl|Sequence
        (:then_0
          (Math|Integer|IncrementInt (Variables|Default|GetTotalItemsSpawned)))
        (:then_1
          (bind _returnvalue (Game|SpawnActorfromClass "/Game/MyGame/BluePrint/Jonino/Item/BP_Item.BP_Item_C" (Math|Transform|MakeTransform (Transformation|GetSocketLocation Static%20mesh%20component _array_element) (Math|Rotator|MakeRotator 0.0 0.0 (.yaw (Math|Random|RandomRotator false))) "1,1,1") "Undefined" 0 0))
          (Variables|/Script/Engine.PrimitiveComponent|SetbGenerateOverlapEvents (Variables|/Game/MyGame/BluePrint/Jonino/Item/BP_Item.BP_Item_C|GetObjectMesh _returnvalue) true)
          (Default|SetRandomMesh _returnvalue true)
          (Utilities|Array|Add (Variables|Default|GetReturnedItems) _returnvalue)))
      (else
        (Utilities|Array|Add (Variables|Default|GetLocationsFurniture) (Transformation|GetSocketLocation Static%20mesh%20component _array_element)))))
  (Utilities|FlowControl|Sequence
    (:then_0
      (return (Variables|Default|GetReturnedItems)))
    (:then_1
      (Utilities|Array|Clear (Variables|Default|GetReturnedItems)))))

(fn GetItemsInteractable
  (params (Static%20mesh%20component :type Static%20Mesh%20Component%20Object%20Reference))
  (for _array_element (Transformation|GetAllSocketNames Static%20mesh%20component)
    (if (Math|Random|RandomBoolwithWeight 0.5)
      (Utilities|FlowControl|Sequence
        (:then_0
          (Math|Integer|IncrementInt (Variables|Default|GetTotalItemsSpawned)))
        (:then_1
          (bind _returnvalue (Game|SpawnActorfromClass "/Game/MyGame/BluePrint/Jonino/Item/BP_Item.BP_Item_C" (Math|Transform|MakeTransform (Transformation|GetSocketLocation Static%20mesh%20component _array_element) (Math|Rotator|MakeRotator 0.0 0.0 (.yaw (Math|Random|RandomRotator false))) "1,1,1") "Undefined" 0 0))
          (Variables|/Script/Engine.PrimitiveComponent|SetbGenerateOverlapEvents (Variables|/Game/MyGame/BluePrint/Jonino/Item/BP_Item.BP_Item_C|GetObjectMesh _returnvalue) false)
          (Default|SetRandomMesh _returnvalue false)
          (Utilities|Array|Add (Variables|Default|GetReturnedItems) _returnvalue)))
      (else
        (Utilities|Array|Add (Variables|Default|GetLocationsInteractable) (Transformation|GetSocketLocation Static%20mesh%20component _array_element)))))
  (Utilities|FlowControl|Sequence
    (:then_0
      (return (Variables|Default|GetReturnedItems)))
    (:then_1
      (Utilities|Array|Clear (Variables|Default|GetReturnedItems)))))