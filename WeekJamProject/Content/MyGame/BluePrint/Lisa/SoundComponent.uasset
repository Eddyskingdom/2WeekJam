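; Blueprint that plays an impact sound at the hit location when its Cube component collides.
; The hit actor's speed is remapped over an inverted range to an integer "power" sound parameter, so slower hits give higher values, and is printed for debugging.
; A DoOnce, reset after a short random delay, throttles repeated hits.
; Fridge variables and a print-only custom event appear to be leftovers.
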(event OnComponentHit(Cube)
  (params (HitComponent :type Primitive%20Component%20Object%20Reference) (OtherActor :type Actor%20Object%20Reference) (OtherComp :type Primitive%20Component%20Object%20Reference) (NormalImpulse :type Vector :default "0, 0, 0") (Hit :type Hit%20Result%20Structure%20%28by%20ref%29))
  (bind (_bblockinghit _binitialoverlap _time _distance _location _impactpoint _normal _impactnormal _physmat _hitactor) (Collision|BreakHitResult Hit))
  (bind _returnvalue (Transformation|GetVelocity _hitactor))
  (bind _returnvalue_2 (Math|Vector|VectorLength _returnvalue))
  (bind _returnvalue_3 (Math|Float|MapRangeClamped _returnvalue_2 9e+01 5.0 0.0 2.0))
  (bind _returnvalue_4 (Math|Float|Truncate _returnvalue_3))
  ;[1 1 1] PlaySoundIfObjectCollides
  (Utilities|FlowControl|Sequence
    (:then_0
      (Utilities|FlowControl|DoOnce false :!label _label
        (:Completed
          (bind _returnvalue_5 (Audio|SpawnSoundatLocation 0 _location "0, 0, 0" 1.0 1.0 0.0 0 0))
          (Effects|Components|ParticleSystem|SetIntParameter _returnvalue_5 "power" _returnvalue_4)
          (Development|PrintString (Utilities|String|ToString(Integer) _returnvalue_4)))))
    (:then_1
      (Utilities|FlowControl|Delay (Math|Random|RandomFloatinRange 0.4 0.6))
      (goto _label Reset))))

(event Custom|CustomEvent
  (params (DeltaSeconds :type Float%20%28single-precision%29))
  (Utilities|Casting|CastToMeshComponent self)
  (Development|PrintString "Hello"))

(event EventBeginPlay)