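; Player character for a timed search game, asleep at the main menu until a wake-up montage sequence enables input, UI and tutorial prompts.
; An interaction sphere gathers items and interactables, ranked each tick by facing dot product, with 2D distance choosing between the two types.
; Montage notifies trigger pickup and physics throws, while UI hints follow context.
; Finding the revolver stops input, and an expired countdown ragdolls the player.
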(event OnComponentEndOverlap(InteractionSphere)
  (params (OverlappedComponent :type Primitive%20Component%20Object%20Reference) (OtherActor :type Actor%20Object%20Reference) (OtherComp :type Primitive%20Component%20Object%20Reference) (OtherBodyIndex :type Integer))
  (bind _itemsinrange (Variables|Item|GetItemsInRange))
  ;[1 1 1] Check For items in range
  (bind _asbp_item (Utilities|Casting|CastToBP_Item OtherActor)
    (:then
      (if (Utilities|Array|ContainsItem _itemsinrange _asbp_item)
        (Utilities|Array|RemoveItem _itemsinrange _asbp_item)))
    (:CastFailed
      (CallFunction|CheckforInteractableRemove OtherActor))))

(event OnComponentBeginOverlap(InteractionSphere)
  (params (OverlappedComponent :type Primitive%20Component%20Object%20Reference) (OtherActor :type Actor%20Object%20Reference) (OtherComp :type Primitive%20Component%20Object%20Reference) (OtherBodyIndex :type Integer) (bFromSweep :type Boolean) (SweepResult :type Hit%20Result%20Structure%20%28by%20ref%29))
  (bind _itemsinrange (Variables|Item|GetItemsInRange))
  ;[1 1 1] Check For items in range
  (bind _asbp_item (Utilities|Casting|CastToBP_Item OtherActor)
    (:then
      (if (not (Utilities|Array|ContainsItem _itemsinrange _asbp_item))
        (Utilities|Array|Add _itemsinrange _asbp_item)))
    (:CastFailed
      (CallFunction|CheckforInteractableAdd OtherActor))))

(event Custom|SetActiveCamera
  (params (NewCamera :type BP%20Follow%20Camera%20Object%20Reference))
  ;[1 1 1] Check Time Input
  (Variables|Default|SetactiveCamera NewCamera))

(event Custom|SetUI
  ;[1 1 1] Create UI and add it to the viewport
  (bind _returnvalue (UserInterface|CreateWidget "/Game/MyGame/UI/WB_IngameUI.WB_IngameUI_C"))
  (bind _output_get (Variables|Default|SetIngameUI _returnvalue))
  (UserInterface|Viewport|AddtoViewport _output_get 0)
  (Default|ShowInteraction (Variables|Default|GetIngameUI) "NewEnumerator0" "Visible")
  (Default|ShowInteraction (Variables|Default|GetIngameUI) "NewEnumerator3" "Visible"))

(event Custom|AddToInView
  (params (Item :type BP%20Item%20Object%20Reference))
  ;[1 1 1] Adding and removing nearby items in view
  (if (not (Utilities|Array|ContainsItem (Variables|Item|GetItemsInView) Item))
    (Utilities|Array|Add (Variables|Item|GetItemsInView) Item)))

(event Custom|CheckForInteractableRemove
  (params (Actor :type Actor%20Object%20Reference))
  ;[1 1 1] Check for interactable in view
  (bind _asbp_interactable (Utilities|Casting|CastToBP_Interactable Actor))
  (Utilities|Array|RemoveItem (Variables|Interactable|GetInteractables) _asbp_interactable))

(event Custom|CheckForInteractableAdd
  (params (Actor :type Actor%20Object%20Reference))
  ;[1 1 1] Check for interactable in view
  (bind _asbp_interactable (Utilities|Casting|CastToBP_Interactable Actor))
  (Utilities|Array|Add (Variables|Interactable|GetInteractables) _asbp_interactable))

(event Custom|Main%20Menu%20Setup
  ;[1 1 1] Main Menu Setup
  (CallFunction|StopPlayerInput)
  (Animation|Montage|PlayMontage (Variables|Character|GetMesh) "/Game/MyGame/Characters/Animations/Montages/Sleeping.Sleeping"))

(event Custom|UpdateNearestInteractable
  (bind _interactablesin_view (Variables|Interactable|GetInteractablesIn_View))
  ;[1 1 1] Check for interactable in view
  (Utilities|FlowControl|Sequence
    (:then_0
      (Variables|Interactable|SethighestDotInteractable 0.0)
      (bind _array_element (Utilities|Array|ForEachLoopwithBreak (Variables|Interactable|GetInteractables))
        (:LoopBody
          (bind (_infront _dot) (CallFunction|IsObjectInfrontOfMe _array_element))
          (if _infront
            (Default|SetDottoPlayer _array_element _dot)
            (Utilities|Array|Add (Variables|Interactable|GetInteractablesIn_View) _array_element)))
        (:Completed
          (for _array_element_2 _interactablesin_view
            (bind _dot_2 (Default|GetDottoPlayer _array_element_2))
            (if (> _dot_2 (Variables|Interactable|GethighestDotInteractable))
              (Variables|Interactable|SetTargetInteractable _array_element_2)))
          (Utilities|Array|Clear _interactablesin_view)
          (if (Utilities|IsValid (Variables|Interactable|GetTargetInteractable))
            (Default|SetTextforInteractable (Variables|Default|GetIngameUI) (Utilities|Text|ToText(Name) (Variables|/Game/MyGame/BluePrint/Jonino/Interactable/Bp_Interactable.BP_Interactable_C|GetObjectNameInRow (Variables|Interactable|GetTargetInteractable))))))))
    (:then_1
      (if (== (Utilities|Array|Length (Variables|Interactable|GetInteractables)) 0)
        (Variables|Interactable|SetTargetInteractable 0)))))

(event Custom|UseInteractable
  (bind _targetinteractable (Variables|Interactable|GetTargetInteractable))
  ;[1 1 1] Pickup/Interact
  (Default|OpenInteractable _targetinteractable)
  (Utilities|Array|RemoveItem (Variables|Interactable|GetInteractables) _targetinteractable)
  (Default|CallInteracted))

(event Custom|WakeUp
  (bind _returnvalue (Transformation|GetActorRotation))
  ;[1 1 1] Main Menu Setup
  (Animation|Montage|PlayMontage (Variables|Character|GetMesh) "/Game/MyGame/Characters/Animations/Montages/Sleeping_Idle__1__Montage.Sleeping_Idle__1__Montage" 1.0 0.0 "Start"
    (:then
      (bind _returnvalue_2 (Actor|GetActorOfClass "/Game/MyGame/BluePrint/Jonino/Managers/BP_CameraManager.BP_CameraManager_C")))
    (:OnBlendOut
      (Default|SwitchCamera _returnvalue_2 "NewEnumerator6")
      (Transformation|SetActorRotation (Math|Rotator|MakeRotator (.roll _returnvalue) (.pitch _returnvalue) -1.8e+02))
      (Transformation|AddActorLocalOffset (* (Transformation|GetActorForwardVector) -1e+02) false true)
      (Animation|Montage|PlayMontage (Variables|Character|GetMesh) "/Game/MyGame/Characters/Animations/Montages/Stand_Up_Montage.Stand_Up_Montage"
        (:OnCompleted
          (Input|EnableInput (Game|GetPlayerController 0))
          (CallFunction|SetUI)
          (CallFunction|PlayerDialogue))
        (:OnNotifyBegin
          (Default|SwitchCamera _returnvalue_2 "NewEnumerator2"))))))

(event Custom|StopPlayerInput
  (Input|DisableInput (Game|GetPlayerController 0)))

(event Custom|PlayerDialogue
  ;[1 1 1] PlayerPrompt
  (Default|SetText (Variables|Default|GetAs%20WB%20Prompt) "I dont have much time, Which I can check by pressing [ T ]")
  (Utilities|FlowControl|Delay 5.0)
  (Default|SetText (Variables|Default|GetAs%20WB%20Prompt) "All Input is shown in the bottom right, which updates depending on my surroundings")
  (Utilities|FlowControl|Delay 5.0)
  (Default|SetText (Variables|Default|GetAs%20WB%20Prompt)))

(event Custom|ShowTimeLeft
  (params (Visibility :type ESlateVisibility%20Enum :default "Visible"))
  (bind _ingameui (Variables|Default|GetIngameUI))
  ;[1 1 1] Check Time Input
  (Default|SetTimeVisibility _ingameui Visibility)
  (Animation|Montage|PlayMontage (Variables|Character|GetMesh) "/Game/MyGame/Characters/Animations/Montages/CheckTime_Montage.CheckTime_Montage" 1.0 0.0 "Start"
    (:OnCompleted
      _)
    (:OnInterrupted
      _))
  (Utilities|FlowControl|Sequence
    (:then_0
      (Utilities|FlowControl|DoOnce false) ; enters at Reset
    )
    (:then_1
      (Default|SetTimeVisibility _ingameui "Hidden"))))

(event Custom|UpdateInteractionInfoUI
  (bind _ingameui (Variables|Default|GetIngameUI))
  (bind _ingameui_2 (Variables|Default|GetIngameUI))
  (bind _ingameui_3 (Variables|Default|GetIngameUI))
  (bind _ingameui_4 (Variables|Default|GetIngameUI))
  (bind _itemtoequip (Variables|Item|GetItemToEquip))
  (bind _targetinteractable (Variables|Interactable|GetTargetInteractable))
  ;[1 1 1] Update Input UI
  (if (not (Variables|Animations|GetinMontage))
    (if (Variables|Item|GethasItemInHand)
      (Default|ShowInteraction _ingameui_4 "NewEnumerator1" "Hidden")
      (Default|ShowInteraction _ingameui_4 "NewEnumerator2" "Visible")
      (Default|ShowInteraction _ingameui_4 "NewEnumerator4" "Hidden")
      (Default|ShowInteraction _ingameui_4 "NewEnumerator3" "Hidden")
      (else
        (Utilities|FlowControl|Sequence
          (:then_0
            (Default|ShowInteraction _ingameui_4 "NewEnumerator3" "Visible"))
          (:then_1
            (if (and (Utilities|IsValid _itemtoequip) (Utilities|IsValid _targetinteractable))
              (bind _useitem (CallFunction|GetClosest _itemtoequip _targetinteractable))
              (if _useitem
                (Default|ShowInteraction _ingameui_3 "NewEnumerator1" "Visible")
                (Default|ShowInteraction _ingameui_3 "NewEnumerator4" "Hidden")
                (else
                  (Default|ShowInteraction _ingameui_3 "NewEnumerator4" "Visible")
                  (Default|ShowInteraction _ingameui_3 "NewEnumerator1" "Hidden")))
              (else
                (Utilities|FlowControl|Sequence
                  (:then_1
                    (Utilities|IsValid (Variables|Item|GetItemToEquip)
                      (:Is%20Valid
                        (Default|ShowInteraction _ingameui_2 "NewEnumerator1" "Visible"))
                      (:Is%20Not%20Valid
                        (Default|ShowInteraction (Variables|Default|GetIngameUI) "NewEnumerator1" "Hidden")))
                    (Default|ShowInteraction _ingameui_2 "NewEnumerator2" "Hidden"))
                  (:then_2
                    (Utilities|IsValid (Variables|Interactable|GetTargetInteractable)
                      (:Is%20Valid
                        (Default|ShowInteraction _ingameui "NewEnumerator4" "Visible"))
                      (:Is%20Not%20Valid
                        (Default|ShowInteraction _ingameui "NewEnumerator4" "Hidden")))))))))))))

(event Custom|Fall
  (bind _bonename (Variables|Default|GetBoneName))
  ;[1 0.1719 0.1719] Ragdoll
  (Class|PhysicalAnimationComponent|SetSkeletalMeshComponent (Variables|Default|GetPhysicalAnimation) (Variables|Character|GetMesh))
  (Class|PhysicalAnimationComponent|ApplyPhysicalAnimationSettingsBelow (Variables|Default|GetPhysicalAnimation) _bonename (Utilities|Struct|MakePhysicalAnimationData true 1e+03 1e+02 1e+03 1e+02) false)
  (Class|SkeletalMeshComponent|SetAllBodiesBelowSimulatePhysics (Variables|Character|GetMesh) _bonename true false)
  (Physics|SetSimulatePhysics (Variables|Character|GetMesh) true)
  (CallFunction|StopPlayerInput))

(event Custom|PickUpItem
  (bind _itemtoequip (Variables|Item|GetItemToEquip))
  ;[1 1 1] Attaching item to hand
  (if (Utilities|Array|ContainsItem (Variables|Item|GetItemsInRange) _itemtoequip)
    (Utilities|Array|RemoveItem (Variables|Item|GetItemsInRange) _itemtoequip)
    (bind _output_get (Variables|Item|SetEquippedItem (Variables|Item|GetItemToEquip)))
    (Utilities|Casting|CastToBP_Revolver _output_get
      (:then
        (Default|CallRevolverFound)
        (Utilities|FlowControl|Sequence
          (:then_0
            (CallFunction|AttachtoHand :!label _label))
          (:then_1
            (CallFunction|StopPlayerInput))))
      (:CastFailed
        (if (Variables|/Game/MyGame/BluePrint/Jonino/Item/BP_Item.BP_Item_C|GetcanBePickedUp _output_get)
          (goto _label)
          (else
            (Default|RemoveItem (Variables|Item|GetEquippedItem))))))))

(event Custom|UpdateItemRange
  ;[1 1 1] Prioritize item to pick up
  (Variables|Item|SethighestDotItem 0.0)
  (bind _array_element (Utilities|Array|ForEachLoopwithBreak (Variables|Item|GetItemsInRange))
    (:LoopBody
      (bind (_infront _dot) (CallFunction|IsObjectInfrontOfMe _array_element))
      (if _infront
        (Default|SetDottoPlayer _array_element _dot)
        (CallFunction|AddtoinView _array_element)
        (else
          (CallFunction|RemovefrominView _array_element))))
    (:Completed
      (if (== (Utilities|Array|Length (Variables|Item|GetItemsInView)) 0)
        (Variables|Item|SetItemToEquip 0)
        (else
          (bind _array_element_2 (Utilities|Array|ForEachLoopwithBreak (Variables|Item|GetItemsInView))
            (:LoopBody
              (bind _dot_2 (Default|GetDottoPlayer _array_element_2))
              (if (> _dot_2 (Variables|Item|GethighestDotItem))
                (Variables|Item|SethighestDotItem _dot_2)
                (Variables|Item|SetItemToEquip _array_element_2)))
            (:Completed
              (Utilities|Array|Clear (Variables|Item|GetItemsInView)))))))))

(event Custom|AttachToHand
  (bind _equippeditem (Variables|Item|GetEquippedItem))
  ;[1 1 1] Attaching item to hand
  (Default|PickedUp _equippeditem)
  (bind _returnvalue (Transformation|AttachComponentToComponent (Variables|/Script/Engine.Actor|GetRootComponent _equippeditem) (Variables|Default|GetRightHandSocket) "RightHand" "SnapToTarget" "SnapToTarget" "SnapToTarget" false))
  (if _returnvalue
    (Variables|Item|SethasItemInHand true)
    (Default|CallPickedUpItem)
    (else
      (Default|RemoveItem (Variables|Item|GetEquippedItem)))))

(event Custom|Throw%20Item
  (bind _equippeditem (Variables|Item|GetEquippedItem))
  (bind _objectmesh (Variables|/Game/MyGame/BluePrint/Jonino/Item/BP_Item.BP_Item_C|GetObjectMesh _equippeditem))
  ;[1 1 1] Item Throwing
  (if (not (Variables|Animations|GetinMontage))
    (Animation|Montage|PlayMontage (Variables|Character|GetMesh) "/Game/MyGame/Characters/Animations/Montages/Throw_Object__1__Montage.Throw_Object__1__Montage" 1.0 0.0 "Start"
      (:then
        (Variables|Animations|SetinMontage true))
      (:OnCompleted
        (Variables|Animations|SetinMontage false))
      (:OnNotifyBegin
        (Transformation|DetachFromActor _equippeditem "KeepWorld" "KeepWorld" "KeepWorld")
        (Physics|SetSimulatePhysics (Variables|/Game/MyGame/BluePrint/Jonino/Item/BP_Item.BP_Item_C|GetObjectMesh _equippeditem) true)
        (Collision|SetCollisionEnabled _objectmesh "QueryAndPhysics")
        (Variables|Item|SethasItemInHand false)
        (Physics|AddImpulse _objectmesh (* (Transformation|GetActorForwardVector) 1e+03) "None" true)
        (Default|CallThrewItem)))))

(event Custom|RemoveFromInView
  (params (Item :type BP%20Item%20Object%20Reference))
  (bind _itemsinview (Variables|Item|GetItemsInView))
  ;[1 1 1] Adding and removing nearby items in view
  (if (Utilities|Array|ContainsItem _itemsinview Item)
    (Utilities|Array|RemoveItem _itemsinview Item)))

(event EventTick
  (params (DeltaSeconds :type Float%20%28single-precision%29))
  (Utilities|IsValid (Variables|Default|GetIngameUI)
    (:Is%20Valid
      (Utilities|FlowControl|Sequence
        (:then_0
          (Utilities|IsValid "/Game/MyGame/UI/WB_IngameUI.WB_IngameUI"
            (:Is%20Valid
              (Default|UpdateTimeLeft (Variables|Default|GetIngameUI) (Variables|Default|GettimeToSearch))
              (bind _output_get (Variables|Default|SettimeToSearch (- (Variables|Default|GettimeToSearch) DeltaSeconds)))
              (if (<= _output_get 0.0)
                (CallFunction|Fall)))))
        (:then_1
          (CallFunction|UpdateItemRange)
          (CallFunction|UpdateNearestInteractable))
        (:then_2
          (CallFunction|UpdateInteractionInfoUI))))))

(event EventBeginPlay
  ;[1 1 1] Setup Player
  (CallFunction|MainMenuSetup)
  (Variables|/Script/Engine.CharacterMovementComponent|SetMaxWalkSpeed (Variables|Character|GetCharacterMovement) (Variables|Default|GetmovementSpeed))
  (Components|Sphere|SetSphereRadius (Variables|Default|GetInteractionSphere) (* (Variables|Default|GetInteractionRangeInMeters) 1e+02) true)
  (bind _aswb_prompt (Utilities|Casting|CastToWB_Prompt (UserInterface|GetWidget (Variables|Default|GetPrompt))))
  (Variables|Default|SetAs%20WB%20Prompt _aswb_prompt))

(event Input|ActionEvents|InputActionScrollUp
  (params (Key :type Key%20Structure :default "None"))
  ;[1 1 1] Camera Zooming Input
  (:Pressed
    (Utilities|IsValid (Variables|Default|GetactiveCamera)
      (:Is%20Valid
        (Default|Zoomin (Variables|Default|GetactiveCamera))))))

(event Input|ActionEvents|InputActionScrollDown
  (params (Key :type Key%20Structure :default "None"))
  ;[1 1 1] Camera Zooming Input
  (:Pressed
    (Utilities|IsValid (Variables|Default|GetactiveCamera)
      (:Is%20Valid
        (Default|ZoomOut (Variables|Default|GetactiveCamera))))))

(event Input|AxisEvents|InputAxisMoveForward
  (params (AxisValue :type Float%20%28single-precision%29))
  ;[1 1 1] Movement
  (if (not (Variables|Animations|GetinMontage))
    (Pawn|Input|AddMovementInput (Math|Vector|GetForwardVector (Math|Rotator|MakeRotator 0.0 0.0 (.yaw (Transformation|GetActorRotation (Variables|Default|GetactiveCamera))))) AxisValue false)))

(event Input|AxisEvents|InputAxisMoveRight
  (params (AxisValue :type Float%20%28single-precision%29))
  ;[1 1 1] Movement
  (if (not (Variables|Animations|GetinMontage))
    (Pawn|Input|AddMovementInput (Math|Vector|GetRightVector (Math|Rotator|MakeRotator 0.0 0.0 (.yaw (Transformation|GetActorRotation (Variables|Default|GetactiveCamera))))) AxisValue false)))

(event Input|KeyboardEvents|T
  (params (Key :type Key%20Structure :default "None"))
  ;[1 1 1] Check Time Input
  (:Pressed
    (if (not (Variables|Animations|GetinMontage))
      (Utilities|FlowControl|DoOnce false
        (:Completed
          (CallFunction|ShowTimeLeft "Visible")
          (Widget|SetVisibility (Variables|Default|GetIngameUI) "Visible"))))))

(event Input|KeyboardEvents|F
  (params (Key :type Key%20Structure :default "None"))
  ;[1 1 1] Pickup/Interact
  (:Pressed
    (if (not (Variables|Animations|GetinMontage))
      (if (Variables|Item|GethasItemInHand)
        (CallFunction|ThrowItem)
        (elif (or (Utilities|IsValid (Variables|Interactable|GetTargetInteractable)) (Utilities|IsValid (Variables|Item|GetItemToEquip)))
          (bind _useitem (CallFunction|GetInteractionChoice))
          (if _useitem
            (CallFunction|ChangePickupAnimation)
            (bind _notifyname (Animation|Montage|PlayMontage (Variables|Character|GetMesh) (Variables|Default|GetMontage%20to%20Play))
              (:then
                (Variables|Animations|SetinMontage true))
              (:OnCompleted
                (Variables|Animations|SetinMontage false))
              (:OnNotifyBegin
                (switch name _notifyname
                  (:Pickup
                    (CallFunction|PickUpItem)))))
            (else
              (CallFunction|UseInteractable))))))))

(event Input|KeyboardEvents|E
  (params (Key :type Key%20Structure :default "None"))
  ;[1 1 1] Pickup/Interact
  (:Pressed
    (if (not (Variables|Animations|GetinMontage))
      (if (Variables|Item|GethasItemInHand)
        (CallFunction|ThrowItem)
        (elif (or (Utilities|IsValid (Variables|Interactable|GetTargetInteractable)) (Utilities|IsValid (Variables|Item|GetItemToEquip)))
          (bind _useitem (CallFunction|GetInteractionChoice))
          (if _useitem
            (CallFunction|ChangePickupAnimation)
            (bind _notifyname (Animation|Montage|PlayMontage (Variables|Character|GetMesh) (Variables|Default|GetMontage%20to%20Play))
              (:then
                (Variables|Animations|SetinMontage true))
              (:OnCompleted
                (Variables|Animations|SetinMontage false))
              (:OnNotifyBegin
                (switch name _notifyname
                  (:Pickup
                    (CallFunction|PickUpItem)))))
            (else
              (CallFunction|UseInteractable))))))))

(event Input|KeyboardEvents|P
  (params (Key :type Key%20Structure))
  (:Pressed
    (Utilities|FlowControl|FlipFlop
      (:A
        (Animation|Montage|PlayMontage (Variables|Character|GetMesh) "/Game/MyGame/Characters/Animations/Montages/Wave_Hip_Hop_Dance_Montage.Wave_Hip_Hop_Dance_Montage")))))

(fn ConstructionScript)

(fn IsObjectInfrontOfMe
  (params (Actor :type Actor%20Object%20Reference))
  (bind _self self)
  (bind _returnvalue (Class|Actor|GetDotProductto _self Actor))
  (return (> _returnvalue 0.2) _returnvalue))

(fn GetInteractionChoice
  (bind _returnvalue (Transformation|GetActorLocation))
  (bind _returnvalue_2 (Transformation|GetActorLocation))
  (bind _targetinteractable (Variables|Interactable|GetTargetInteractable))
  (bind _itemtoequip (Variables|Item|GetItemToEquip))
  (bind _returnvalue_3 (Transformation|GetActorLocation _targetinteractable))
  (bind _returnvalue_4 (Transformation|GetActorLocation _itemtoequip))
  (if (and (Utilities|IsValid (Variables|Interactable|GetTargetInteractable)) (Utilities|IsValid (Variables|Item|GetItemToEquip)))
    (return (> (Math|Vector|Distance(Vector) (Math|Vector|MakeVector (.x _returnvalue_3) (.y _returnvalue_3) 0.0) (Math|Vector|MakeVector (.x _returnvalue_2) (.y _returnvalue_2) 0.0)) (Math|Vector|Distance(Vector) (Math|Vector|MakeVector (.x _returnvalue_4) (.y _returnvalue_4) 0.0) (Math|Vector|MakeVector (.x _returnvalue) (.y _returnvalue) 0.0))))
    (elif (Utilities|IsValid (Variables|Item|GetItemToEquip))
      (return true)
      (elif (Utilities|IsValid (Variables|Interactable|GetTargetInteractable))
        (return false)))))

(fn GetClosest
  (params (Item :type Actor%20Object%20Reference) (Interactable :type Actor%20Object%20Reference))
  (bind _returnvalue (Transformation|GetActorLocation))
  (bind _returnvalue_2 (Transformation|GetActorLocation))
  (bind _returnvalue_3 (Transformation|GetActorLocation Interactable))
  (bind _returnvalue_4 (Transformation|GetActorLocation Item))
  (return (< (Math|Vector|Distance(Vector) (Math|Vector|MakeVector (.x _returnvalue) (.y _returnvalue) 0.0) (Math|Vector|MakeVector (.x _returnvalue_4) (.y _returnvalue_4) 0.0)) (Math|Vector|Distance(Vector) (Math|Vector|MakeVector (.x _returnvalue_2) (.y _returnvalue_2) 0.0) (Math|Vector|MakeVector (.x _returnvalue_3) (.y _returnvalue_3) 0.0)))))

(fn ChangePickupAnimation
  (if (> (+ (.z (Transformation|GetActorLocation (Variables|Item|GetItemToEquip))) (LocalVariables|GetOffset)) (.z (Transformation|GetActorLocation)))
    (Variables|Default|SetMontage%20to%20Play "/Game/MyGame/Characters/Animations/Montages/PickupItem_Montage.PickupItem_Montage")
    (else
      (Variables|Default|SetMontage%20to%20Play "/Game/MyGame/Characters/Animations/Montages/PickupItem_Montage.PickupItem_Montage"))))